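; BP_Patient is a clickable patient actor that has a condition and a critical state.
; Clicking it prints the condition and stores the actor as SelectedPatient on BP_ThirdPersonPlayerController, with debug prints confirming the click and selection.
; The IsStable function reports stability as the inverse of IsCritical.
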(event EventBeginPlay)

(event Collision|EventActorBeginOverlap
  (params (OtherActor :type Actor%20Object%20Reference)))

(event EventTick
  (params (DeltaSeconds :type Float%20%28single-precision%29)))

(event MouseInput|EventActorOnClicked
  (params (ButtonPressed :type Key%20Structure :default "None"))
  (Development|PrintString "Patient Clicked")
  (Development|PrintString (Utilities|String|ToString(Text) (Utilities|Text|FormatText "Condition: {Cond}" (Variables|Default|GetCondition))))
  (bind _asbp_third_person_player_controller (Utilities|Casting|CastToBP_ThirdPersonPlayerController (Game|GetPlayerController 0)))
  (Variables|/Game/ThirdPerson/Blueprints/BP_ThirdPersonPlayerController.BP_ThirdPersonPlayerController_C|SetSelectedPatient _asbp_third_person_player_controller self)
  (Development|PrintString "Selected patient saved"))

(fn ConstructionScript)

(fn IsStable
  (return (not (Variables|Default|GetIsCritical))))