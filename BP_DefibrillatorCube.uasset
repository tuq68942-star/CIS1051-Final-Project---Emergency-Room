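; Clickable defibrillator actor that treats the player controller's selected patient in a medical triage game.
; A click clears a critical Cardiac Arrest patient's critical state and updates the UI message, printing errors for invalid uses.
; It then scans all BP_Patient actors, adding to a never-reset StableCount for the UI counter.
; When none remain critical, it shows the win widget and opens Lvl_ThirdPerson after a delay.
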(event EventBeginPlay)

(event Collision|EventActorBeginOverlap
  (params (OtherActor :type Actor%20Object%20Reference)))

(event EventTick
  (params (DeltaSeconds :type Float%20%28single-precision%29)))

(event MouseInput|EventActorOnClicked
  (params (ButtonPressed :type Key%20Structure :default "None"))
  (Development|PrintString "Defribrilator Clicked")
  (bind _asbp_third_person_player_controller (Utilities|Casting|CastToBP_ThirdPersonPlayerController (Game|GetPlayerController 0)))
  (Utilities|IsValid (Variables|/Game/ThirdPerson/Blueprints/BP_ThirdPersonPlayerController.BP_ThirdPersonPlayerController_C|GetSelectedPatient _asbp_third_person_player_controller)
    (:Is%20Valid
      (if (Variables|/Game/Characters/Mannequins/Meshes/BP_Patient.BP_Patient_C|GetIsCritical (Variables|/Game/ThirdPerson/Blueprints/BP_ThirdPersonPlayerController.BP_ThirdPersonPlayerController_C|GetSelectedPatient _asbp_third_person_player_controller))
        (if (Utilities|Enum|Equal(Enum) (Variables|/Game/Characters/Mannequins/Meshes/BP_Patient.BP_Patient_C|GetCondition (Variables|/Game/ThirdPerson/Blueprints/BP_ThirdPersonPlayerController.BP_ThirdPersonPlayerController_C|GetSelectedPatient _asbp_third_person_player_controller)) "Cardiac Arrest")
          (Default|UpdateMessage (Variables|/Game/ThirdPerson/Blueprints/BP_ThirdPersonPlayerController.BP_ThirdPersonPlayerController_C|GetGameUIRef _asbp_third_person_player_controller) "Patient stablized: heart rate normal")
          (Variables|/Game/Characters/Mannequins/Meshes/BP_Patient.BP_Patient_C|SetIsCritical (Variables|/Game/ThirdPerson/Blueprints/BP_ThirdPersonPlayerController.BP_ThirdPersonPlayerController_C|GetSelectedPatient _asbp_third_person_player_controller) false)
          (Variables|Default|SetAllPatientsStable true)
          (bind _outactors (Actor|GetAllActorsOfClass "/Game/Characters/Mannequins/Meshes/BP_Patient.BP_Patient_C"))
          (for _array_element _outactors
            (bind _asbp_patient (Utilities|Casting|CastToBP_Patient _array_element))
            (if (Variables|/Game/Characters/Mannequins/Meshes/BP_Patient.BP_Patient_C|GetIsCritical _asbp_patient)
              (Variables|Default|SetAllPatientsStable false)
              (else
                (Variables|Default|SetStableCount (+ (Variables|Default|GetStableCount) 1)))))
          (bind _asbp_third_person_player_controller_2 (Utilities|Casting|CastToBP_ThirdPersonPlayerController (Game|GetPlayerController 0)))
          (Default|UpdateStableCounter (Variables|/Game/ThirdPerson/Blueprints/BP_ThirdPersonPlayerController.BP_ThirdPersonPlayerController_C|GetGameUIRef _asbp_third_person_player_controller_2) (Variables|Default|GetStableCount))
          (if (Variables|Default|GetAllPatientsStable)
            (Development|PrintString "You Win")
            (bind _returnvalue (UserInterface|CreateWidget "/Game/UI/WBP_YouWin.WBP_YouWin_C" (Game|GetPlayerController 0)))
            (UserInterface|Viewport|AddtoViewport _returnvalue 0)
            (Utilities|FlowControl|Delay 2.0)
            (Game|OpenLevel(byName) "Lvl_ThirdPerson"))
          (else
            (Development|PrintString "Wrong Treatment")))
        (else
          (Development|PrintString "Do Not Shcok Stable Patient"))))
    (:Is%20Not%20Valid
      (Development|PrintString "No Patient Selected"))))

(fn ConstructionScript)